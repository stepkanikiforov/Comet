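; Pawn Blueprint for the comet, which applies the skin color stored in the game instance to its skeletal mesh.
; The Construction Script casts to CometGameInstance and uses SkinColor to set the first material slot to pink, yellow or the default MasterMaterial.
; The Event Graph holds only a debug print on touch press, alongside disabled stub events.
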(event EventBeginPlay)

(event Collision|EventActorBeginOverlap
  (params (OtherActor :type Actor%20Object%20Reference)))

(event EventTick
  (params (DeltaSeconds :type Float%20%28single-precision%29)))

(event Input|TouchEvents|InputTouch
  (params (Location :type Vector) (FingerIndex :type ETouchIndex%20Enum))
  (:Pressed
    (Development|PrintString "Hello")))

(fn ConstructionScript
  (bind _ascomet_game_instance (Utilities|Casting|CastToCometGameInstance (Game|GetGameInstance)))
  (if (== (Variables|/Script/Comet.CometGameInstance|GetSkinColor _ascomet_game_instance) 2)
    (Rendering|Material|SetMaterial (Variables|Default|GetSkeletalMesh) 0 "/Game/Materials/MI_PawnPink.MI_PawnPink")
    (elif (== (Variables|/Script/Comet.CometGameInstance|GetSkinColor _ascomet_game_instance) 3)
      (Rendering|Material|SetMaterial (Variables|Default|GetSkeletalMesh) 0 "/Game/Materials/MI_PawnYellow.MI_PawnYellow")
      (else
        (Rendering|Material|SetMaterial (Variables|Default|GetSkeletalMesh) 0 "/Game/Materials/MasterMaterial.MasterMaterial")))))